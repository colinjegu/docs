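; Stylized explosion VFX actor that fires one second after BeginPlay and replays when A is pressed.
; It spawns an anticipation Niagara system, waits briefly, then starts a camera shake and spawns the red explosion system.
; A sped-up timeline drives the Alpha parameter in MPC_Explosion and resets global time dilation to normal when finished.
; The timeline-driven time dilation node is left unwired, so no slow motion occurs.
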(event `self.ReceiveBeginPlay`
  (`KismetSystemLibrary.K2_SetTimerDelegate` (delegate `Bomb`) 1.0))

(event `Bomb`
  (`NiagaraFunctionLibrary.SpawnSystemAtLocation` null "/Game/Core/VFX/StylizedExplosion/NS_Anticipation.NS_Anticipation" :!label _label)
  (`KismetSystemLibrary.Delay` null 0.4)
  (`CameraShakeSourceComponent.Start` (`self.CameraShakeSource`))
  (`TimelineComponent.SetPlayRate` (`self.Timeline`) 10.0)
  (`|ExecutionSequence`
    (:`then_0`
      (bind (_direction _alpha) (`Timeline|Timeline` :!via `PlayFromStart`)
        (:`Update`
          (`|ExecutionSequence`
            (:`then_1`
              (`KismetMaterialLibrary.SetScalarParameterValue` null "/Game/Core/VFX/StylizedExplosion/MPC_Explosion.MPC_Explosion" "Alpha" _alpha))))
        (:`Finished`
          (`GameplayStatics.SetGlobalTimeDilation` null 1.0))))
    (:`then_1`
      (`NiagaraFunctionLibrary.SpawnSystemAtLocation` null "/Game/Core/VFX/StylizedExplosion/NS_StylizedExplosion_Red.NS_StylizedExplosion_Red"))))

(event `Key|A`
  (params (Key :type "Key Structure"))
  (:`Pressed`
    (goto _label)))

(fn `UserConstructionScript`
  (`self.EditorTickEnabled`)
  (`self.SetActorTickEnabled` true))