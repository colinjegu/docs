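; A player-controlled pawn for firing stylized Niagara explosions, with look, planar and vertical movement through Enhanced Input.
; Shooting line-traces from the camera; a hit spawns an anticipation effect, then after a short delay a randomly scaled red explosion at that point.
; A miss spawns the explosion immediately without a specified location.
; Both paths start a camera shake and a sped-up timeline that drives Alpha in the MPC_Explosion material parameter collection.
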(event `EnhancedInput|/Game/Core/EnhancedInput/Input/Actions/IA_Look`
  (params (ActionValue :type "Vector2D Structure") (ElapsedSeconds :type "Float (double-precision)") (TriggeredSeconds :type "Float (double-precision)") (InputAction :type "InputAction Object Reference" :default "/Game/Core/EnhancedInput/Input/Actions/IA_Look.IA_Look"))
  (:`Triggered`
    (`self.AddControllerYawInput` ActionValue_X)
    (`self.AddControllerPitchInput` ActionValue_Y)))

(event `EnhancedInput|/Game/Core/EnhancedInput/Input/Actions/IA_Move`
  (params (ActionValue :type "Vector2D Structure") (ElapsedSeconds :type "Float (double-precision)") (TriggeredSeconds :type "Float (double-precision)") (InputAction :type "InputAction Object Reference" :default "/Game/Core/EnhancedInput/Input/Actions/IA_Move.IA_Move"))
  (bind _camera (`self.Camera`))
  (:`Triggered`
    (`self.AddMovementInput` (`SceneComponent.GetRightVector` _camera) ActionValue_X)
    (`self.AddMovementInput` (`SceneComponent.GetForwardVector` _camera) ActionValue_Y)))

(event `EnhancedInput|/Game/Core/EnhancedInput/Input/Actions/IA_Up`
  (params (ActionValue :type "Vector2D Structure") (ElapsedSeconds :type "Float (double-precision)") (TriggeredSeconds :type "Float (double-precision)") (InputAction :type "InputAction Object Reference" :default "/Game/Core/EnhancedInput/Input/Actions/IA_Up.IA_Up"))
  (:`Triggered`
    (`self.AddMovementInput` (`self.GetActorUpVector`) ActionValue_X)
    (`self.AddMovementInput` (`self.GetActorUpVector`) ActionValue_Y)))

(event `EnhancedInput|/Game/Core/EnhancedInput/Input/Actions/IA_Shoot`
  (params (ActionValue :type Boolean) (ElapsedSeconds :type "Float (double-precision)") (TriggeredSeconds :type "Float (double-precision)") (InputAction :type "InputAction Object Reference" :default "/Game/Core/EnhancedInput/Input/Actions/IA_Shoot.IA_Shoot"))
  (bind _returnvalue (`SceneComponent.K2_GetComponentLocation` (`self.Camera`)))
  (:`Started`
    (bind _outhit (`KismetSystemLibrary.LineTraceSingle` _returnvalue (+ _returnvalue (* (`SceneComponent.GetForwardVector` (`self.Camera`)) (`KismetMathLibrary.Conv_DoubleToVector` 100000.0))) "TraceTypeQuery1"))
    (if (`GameplayStatics.BreakHitResult` _outhit)
      (`NiagaraFunctionLibrary.SpawnSystemAtLocation` "/Game/Core/VFX/StylizedExplosion/NS_Anticipation.NS_Anticipation" (`.Location` (`GameplayStatics.BreakHitResult` _outhit)) (struct) (100.0 100.0 100.0))
      (`KismetSystemLibrary.Delay` 0.4)
      (`NiagaraFunctionLibrary.SpawnSystemAtLocation` "/Game/Core/VFX/StylizedExplosion/NS_StylizedExplosion_Red.NS_StylizedExplosion_Red" (`.Location` (`GameplayStatics.BreakHitResult` _outhit)) (struct) (`KismetMathLibrary.Conv_DoubleToVector` (`KismetMathLibrary.RandomFloatInRange` 0.8 1.2)))
      (`CameraShakeSourceComponent.Start` (`self.CameraShakeSource`))
      (`TimelineComponent.SetPlayRate` (`self.Alpha`) 10.0)
      (bind (_direction _alpha) (`Timeline|Alpha` :!via `PlayFromStart`)
        (:`Update`
          (`KismetMaterialLibrary.SetScalarParameterValue` "/Game/Core/VFX/StylizedExplosion/MPC_Explosion.MPC_Explosion" "Alpha" _alpha)))
      (else
        (`NiagaraFunctionLibrary.SpawnSystemAtLocation` "/Game/Core/VFX/StylizedExplosion/NS_StylizedExplosion_Red.NS_StylizedExplosion_Red")
        (`CameraShakeSourceComponent.Start` (`self.CameraShakeSource`))
        (`TimelineComponent.SetPlayRate` (`self.Timeline`) 10.0)
        (bind (_direction_2 _alpha_2) (`Timeline|Timeline` :!via `PlayFromStart`)
          (:`Update`
            (`KismetMaterialLibrary.SetScalarParameterValue` "/Game/Core/VFX/StylizedExplosion/MPC_Explosion.MPC_Explosion" "Alpha" _alpha_2)))))))

(event `Key|A`
  (params (Key :type "Key Structure")))

(fn `UserConstructionScript`)