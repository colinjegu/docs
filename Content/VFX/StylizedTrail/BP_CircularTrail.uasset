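; BP_CircularTrail is an actor that moves a Niagara effect in a circle around its origin, in game and in the editor.
; Construction assigns the chosen Effect asset and enables editor and actor ticking.
; Both ticks share one update that derives delta time from game time since creation, skips large time steps, and sets the component's relative location with sine and cosine, scaled by Speed and Radius.
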(event `/Game/Core/Editor/BPI_EditorTick.EditorTick`
  (bind _returnvalue (`self.GetGameTimeSinceCreation`))
  (bind _returnvalue_2 (* (`self.TotalTime`) (`self.Speed`) 360.0))
  ;[0.2812 0.2812 0.2812] Editor Tick only
  (set `self.CurDeltaTime` (- _returnvalue (`self.LastTime`)) :!label _label)
  (set `self.LastTime` _returnvalue)
  (if (< (`self.CurDeltaTime`) 0.04)
    (set `self.TotalTime` (+ (`self.TotalTime`) (`self.CurDeltaTime`)))
    (`SceneComponent.K2_SetRelativeLocation` (`self.Niagara`) (* (`KismetMathLibrary.MakeVector` (`KismetMathLibrary.DegSin` _returnvalue_2) (`KismetMathLibrary.DegCos` _returnvalue_2)) (`self.Radius`)) false false)))

(event `self.ReceiveTick`
  (params (DeltaSeconds :type "Float (single-precision)"))
  (goto _label))

(fn `UserConstructionScript`
  (`NiagaraComponent.SetAsset` (`self.Niagara`) (`self.Effect`) true)
  (`self.EditorTickEnabled`)
  (`self.SetActorTickEnabled` true))