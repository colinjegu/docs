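; Stylized explosion demo actor that fires one second after BeginPlay and replays on the A key.
; It spawns an anticipation Niagara effect, then after a short delay starts camera shake and the red explosion effect.
; A sped-up Timeline drives the Alpha parameter in MPC_StylizedExplosion.
; Every BP_Dummy receives an impulse pointing away from world origin, rather than this actor's location, and has its Physic function called.
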(event `self.ReceiveBeginPlay`
  (`KismetSystemLibrary.K2_SetTimerDelegate` (delegate `Bomb`) 1.0))

(event `Bomb`
  (`NiagaraFunctionLibrary.SpawnSystemAtLocation` null "/Game/VFX/StylizedExplosion/NS_Anticipation.NS_Anticipation" :!label _label)
  (`KismetSystemLibrary.Delay` null 0.4)
  (`CameraShakeSourceComponent.Start` (`self.CameraShakeSource`))
  (`TimelineComponent.SetPlayRate` (`self.Timeline`) 8.0)
  (`|ExecutionSequence`
    (:`then_0`
      (bind (_direction _alpha) (`Timeline|Timeline` :!via `PlayFromStart`)
        (:`Update`
          (`KismetMaterialLibrary.SetScalarParameterValue` null "/Game/VFX/StylizedExplosion/MPC_StylizedExplosion.MPC_StylizedExplosion" "Alpha" _alpha))))
    (:`then_1`
      (`NiagaraFunctionLibrary.SpawnSystemAtLocation` null "/Game/VFX/StylizedExplosion/NS_StylizedExplosion_Red.NS_StylizedExplosion_Red")
      (bind _outactors (`GameplayStatics.GetAllActorsOfClass` null "/Game/VFX/StylizedExplosion/BP_Dummy.BP_Dummy_C"))
      (for _array_element _outactors
        (set `/Game/VFX/StylizedExplosion/BP_Dummy.Impulse` (* (`KismetMathLibrary.GetDirectionUnitVector` (`self.K2_GetActorLocation` _array_element)) (`KismetMathLibrary.Conv_DoubleToVector` -10000.0)) _array_element)
        (`/Game/VFX/StylizedExplosion/BP_Dummy.Physic` _array_element)))))

(event `Key|A`
  (params (Key :type "Key Structure"))
  (:`Pressed`
    (goto _label)))

(fn `UserConstructionScript`
  (`self.EditorTickEnabled`)
  (`self.SetActorTickEnabled` true))