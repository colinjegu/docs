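; BP_Trail is a projectile actor that carries a Niagara trail and knocks back BP_Dummy targets on contact.
; On BeginPlay it copies the trail and impact effects from the BP_Attack found in the level.
; When its sphere overlaps a dummy, it calls Physic with a forward push, spawns the impact at negated rotation and stops moving.
; The actor destroys itself after a short delay following the hit.
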(event `self.ReceiveBeginPlay`
  (bind _returnvalue (`GameplayStatics.GetActorOfClass` "/Game/VFX/StylizedElements/BP_Attack.BP_Attack_C"))
  (set `self.Impact` (`/Game/VFX/StylizedElements/BP_Attack.Impact` _returnvalue))
  (`NiagaraComponent.SetAsset` (`self.Niagara`) (`/Game/VFX/StylizedElements/BP_Attack.Trail` _returnvalue) true))

(event `self.Sphere.OnComponentBeginOverlap`
  (params (OverlappedComponent :type "PrimitiveComponent Object Reference") (OtherActor :type "Actor Object Reference") (OtherComp :type "PrimitiveComponent Object Reference") (OtherBodyIndex :type Integer) (bFromSweep :type Boolean) (SweepResult :type "HitResult Structure (by ref)"))
  (bind _asbp_dummy (cast `/Game/VFX/StylizedElements/BP_Dummy` OtherActor))
  (`/Game/VFX/StylizedElements/BP_Dummy.Physic` _asbp_dummy (* (`KismetMathLibrary.GetForwardVector` (`self.K2_GetActorRotation`)) 5000.0))
  (`NiagaraFunctionLibrary.SpawnSystemAtLocation` (`self.Impact`) (`self.K2_GetActorLocation`) (* (`self.K2_GetActorRotation`) -1.0))
  (`MovementComponent.StopMovementImmediately` (`self.ProjectileMovement`))
  (`KismetSystemLibrary.Delay` 4.0)
  (`self.K2_DestroyActor`))

(fn `UserConstructionScript`)