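; BP_Attack is an emitter actor that repeatedly fires a stylized elemental VFX attack.
; On BeginPlay it looks up its element's row in DTElements for Burst, Trail, Impact and Material, and starts a looping timer on Attack.
; After a short delay, Attack spawns the Burst system and a BP_Trail actor at its own transform, passing on Trail and Impact.
; Material is stored but unused in these graphs.
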(event `self.ReceiveBeginPlay`
  (`self.Attack`)
  (`KismetSystemLibrary.K2_SetTimerDelegate` (delegate `Attack`) 2.0 true)
  (bind _returnvalue (`|GetDataTableRow` (`self.DTElements`) (`KismetStringLibrary.Conv_StringToName` (`|GetEnumeratorNameAsString` (`self.Elements`))))
    (:`then`
      (bind (_burst _trail _impact _material) (break `/Game/VFX/StylizedElements/S_Elements` _returnvalue))
      (set `self.Burst` _burst)
      (set `self.Trail` _trail)
      (set `self.Impact` _impact)
      (set `self.Material` _material))))

(event `Attack`
  (`KismetSystemLibrary.Delay` 0.5)
  (`NiagaraFunctionLibrary.SpawnSystemAtLocation` (`self.Burst`) (`self.K2_GetActorLocation`) (`self.K2_GetActorRotation`))
  (bind _returnvalue (`|SpawnActorFromClass` "/Game/VFX/StylizedElements/BP_Trail.BP_Trail_C" (`KismetMathLibrary.MakeTransform` (`self.K2_GetActorLocation`) (`self.K2_GetActorRotation`)) "Undefined" "OverrideRootScale" null null))
  (set `/Game/VFX/StylizedElements/BP_Trail.Trail` (`self.Trail`) _returnvalue)
  (set `/Game/VFX/StylizedElements/BP_Trail.Impact` (`self.Impact`) _returnvalue))

(fn `UserConstructionScript`)