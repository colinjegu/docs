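; BP_Dummy is a skeletal mesh dummy in the StylizedBeam VFX folder that fakes a reaction to a beam on BeginPlay.
; After a short delay it starts a camera shake and two randomly timed looping timers.
; Both timers enable physics and jolt bodies below bone Main3 with random horizontal impulses until cleared two seconds later.
; In parallel, a timeline drives the mesh materials' Alpha parameter from the start.
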(event `self.ReceiveBeginPlay`
  (`|ExecutionSequence`
    (:`then_0`
      (`KismetSystemLibrary.Delay` 0.5)
      (`CameraShakeSourceComponent.StartCameraShake` :`self` (`self.CameraShakeSource`) :`InCameraShake` "/Game/VFX/StylizedBeam/CS_Beam.CS_Beam_C" :`Scale` 0.5)
      (bind _returnvalue (`KismetSystemLibrary.K2_SetTimerDelegate` (delegate `Physic1`) (`KismetMathLibrary.RandomFloatInRange` 0.1 0.2) true))
      (bind _returnvalue_2 (`KismetSystemLibrary.K2_SetTimerDelegate` (delegate `Physic2`) (`KismetMathLibrary.RandomFloatInRange` 0.1 0.2) true))
      (`KismetSystemLibrary.Delay` 2.0)
      (`KismetSystemLibrary.K2_ClearAndInvalidateTimerHandle` _returnvalue)
      (`KismetSystemLibrary.K2_ClearAndInvalidateTimerHandle` _returnvalue_2))
    (:`then_1`
      (bind (_direction _alpha) (`Timeline|Timeline` :!via `PlayFromStart`)
        (:`Update`
          (`MeshComponent.SetScalarParameterValueOnMaterials` (`self.SkeletalMesh`) "Alpha" _alpha))))))

(event `Physic1`
  (bind _skeletalmesh (`self.SkeletalMesh`))
  (`PrimitiveComponent.SetSimulatePhysics` _skeletalmesh true)
  (`SkeletalMeshComponent.AddImpulseToAllBodiesBelow` _skeletalmesh (* (* (`KismetMathLibrary.RandomUnitVector`) (1.0 1.0 0.0)) (`KismetMathLibrary.Conv_DoubleToVector` 500.0)) "Main3" false true))

(event `Physic2`
  (bind _skeletalmesh (`self.SkeletalMesh`))
  (`PrimitiveComponent.SetSimulatePhysics` _skeletalmesh true)
  (`SkeletalMeshComponent.AddImpulseToAllBodiesBelow` _skeletalmesh (* (* (`KismetMathLibrary.RandomUnitVector`) (1.0 1.0 0.0)) (`KismetMathLibrary.Conv_DoubleToVector` 500.0)) "Main3" false true))

(fn `UserConstructionScript`)