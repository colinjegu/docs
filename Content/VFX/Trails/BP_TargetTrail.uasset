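; Preview-style trail actor that repeatedly moves a Niagara effect in a straight line from its origin to TargetPosition.
; Construction assigns the Effect asset, enables ticking and places the Target component at the endpoint.
; Editor and game ticks share one path that accumulates time, ignoring steps of 0.04 seconds or longer.
; LoopTime and LoopDelay shape the lerp alpha, which wraps to the origin for the delay portion.
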(event `/Game/Core/Editor/BPI_EditorTick.EditorTick`
  (bind _returnvalue (`self.GetGameTimeSinceCreation`))
  ;[0.2812 0.2812 0.2812] Editor Tick only
  (set `self.CurDeltaTime` (- _returnvalue (`self.LastTime`)) :!label _label)
  (set `self.LastTime` _returnvalue)
  (if (< (`self.CurDeltaTime`) 0.04)
    (set `self.TotalTime` (+ (`self.TotalTime`) (`self.CurDeltaTime`)))
    (`SceneComponent.K2_SetRelativeLocation` (`self.Niagara`) (`KismetMathLibrary.VLerp` (0.0 0.0 0.0) (`self.TargetPosition`) (`KismetMathLibrary.Fraction` (`KismetMathLibrary.FClamp` (* (`KismetMathLibrary.Fraction` (/ (`self.TotalTime`) (`self.LoopTime`))) (+ 1.0 (/ (`self.LoopDelay`) (`self.LoopTime`))))))) false false)))

(event `self.ReceiveTick`
  (params (DeltaSeconds :type "Float (single-precision)"))
  (goto _label))

(fn `UserConstructionScript`
  (`NiagaraComponent.SetAsset` (`self.Niagara`) (`self.Effect`) true)
  (`self.EditorTickEnabled`)
  (`self.SetActorTickEnabled` true)
  (`SceneComponent.K2_SetRelativeLocation` (`self.Target`) (`self.TargetPosition`) false false))